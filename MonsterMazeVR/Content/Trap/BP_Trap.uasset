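; BP_Trap is a trap actor that immobilizes a VR player who walks into it.
; On overlap with a VRPlayerPawn it clears the pawn's CanMove flag, then restores it after a three-second delay.
; BeginPlay caches its WBP_Trap widget, but the looping timer meant to poll that widget's IsActivate into TrapActive is unconnected, so the trap fires regardless of activation state.
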(event EventBeginPlay
  (bind _aswbp_trap (Utilities|Casting|CastToWBP_Trap (UserInterface|GetWidget (Variables|Default|GetWidget))))
  (Variables|Default|SetAs%20WBP%20Trap _aswbp_trap))

(event Collision|EventActorBeginOverlap
  (params (OtherActor :type Actor%20Object%20Reference))
  (Utilities|FlowControl|Sequence
    (:then_0
      (bind _asvrplayer_pawn (Utilities|Casting|CastToVRPlayerPawn OtherActor))
      (Variables|/Game/VRTemplate/Blueprints/VRPlayerPawn.VRPlayerPawn_C|SetCanMove _asvrplayer_pawn false)
      (Utilities|FlowControl|Delay 3.0)
      (Variables|/Game/VRTemplate/Blueprints/VRPlayerPawn.VRPlayerPawn_C|SetCanMove _asvrplayer_pawn true))))

(fn ConstructionScript)

(fn CheckActive
  (Variables|Default|SetTrapActive (Variables|/Game/Trap/WBP_Trap.WBP_Trap_C|GetIsActivate (Variables|Default|GetAs%20WBP%20Trap))))