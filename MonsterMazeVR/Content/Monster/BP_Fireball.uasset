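; BP_Fireball is a monster fireball actor that homes in on the player pawn and can be shot down.
; Each tick it moves along its static mesh's forward vector at constant speed without sweeping, while gradually interpolating its rotation toward the player.
; Overlapping a Projectile actor destroys it; no damage to the player is handled here.
; BeginPlay caches the first BP_TestPawn, which the graph never uses.
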(event EventBeginPlay
  (bind _outactors (Actor|GetAllActorsOfClass "/Game/Monster/BP_TestPawn.BP_TestPawn_C"))
  (Variables|Default|SetTest (Utilities|Array|Get(acopy) _outactors)))

(event Collision|EventActorBeginOverlap
  (params (OtherActor :type Actor%20Object%20Reference))
  (Utilities|Casting|CastToProjectile OtherActor)
  (Actor|DestroyActor))

(event EventTick
  (params (DeltaSeconds :type Float%20%28single-precision%29))
  (Transformation|AddActorWorldOffset (* (Math|Vector|GetForwardVector (Variables|Default|GetStaticMesh)) (* DeltaSeconds 5e+02)))
  (Transformation|SetActorRotation (Math|Interpolation|RInterpTo (Transformation|GetActorRotation) (Math|Rotator|FindLookatRotation (Transformation|GetActorLocation) (Transformation|GetActorLocation (Game|Player|GetPlayerPawn 0))) DeltaSeconds 1.0)))

(fn ConstructionScript)