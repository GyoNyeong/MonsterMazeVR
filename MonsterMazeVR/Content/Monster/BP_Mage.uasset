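; BP_Mage is a monster pawn that attacks with volleys of fireballs.
; Every tick it smoothly rotates to face player 0's pawn.
; Once possessed by a BP_MonsterBP controller, it runs a looping timer that polls the blackboard's Monster state enum every few seconds.
; In the Attack state, it plays the attack montage and immediately spawns BP_Fireball actors at three component transforms.
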(event EventBeginPlay
  (|CallParentFunction)
  (bind _asbp_monster_bp (Utilities|Casting|CastToBP_MonsterBP (Pawn|GetController))))

(event Collision|EventActorBeginOverlap
  (params (OtherActor :type Actor%20Object%20Reference))
  (|CallParentFunction OtherActor) ; This node is disabled and will not be called.\nDrag off pins to build functionality.
)

(event EventTick
  (params (DeltaSeconds :type Float%20%28single-precision%29))
  (|CallParentFunction DeltaSeconds)
  (Transformation|SetActorRotation (Math|Interpolation|RInterpTo (Transformation|GetActorRotation) (Math|Rotator|FindLookatRotation (Transformation|GetActorLocation) (Transformation|GetActorLocation (Game|Player|GetPlayerPawn 0))) DeltaSeconds 1.0)))

(event EventPossessed
  (params (NewController :type Controller%20Object%20Reference))
  (Utilities|Casting|CastToBP_MonsterBP NewController)
  (Utilities|Time|SetTimerbyFunctionName 0 "UpdateAiTick" 3.0 true))

(fn ConstructionScript
  (|CallParentFunction))

(fn UpdateAiTick
  (bind _asbp_monster_bp (Utilities|Casting|CastToBP_MonsterBP (Pawn|GetController)))
  (Utilities|IsValid (AI|GetBlackboard _asbp_monster_bp)
    (:Is%20Valid
      (bind _output_get (Variables|Default|SetMonsterState (Utilities|Enum|ByteToEnumEN_Monster (Class|BlackboardComponent|GetValueasEnum (AI|GetBlackboard _asbp_monster_bp) (Utilities|Name|MakeLiteralName "Monster")))))
      (switch Utilities|FlowControl|Switch|SwitchonEN_Monster _output_get
        (:NewEnumerator2
          (Animation|PlayAnimMontage (Variables|Default|GetAttackMontage) 1.0 "None")
          (CallFunction|SpawnFireballs))))))

(fn SpawnFireballs
  (Utilities|FlowControl|Sequence
    (:then_0
      (Game|SpawnActorfromClass "/Game/Monster/BP_Fireball.BP_Fireball_C" (Transformation|GetWorldTransform (Variables|Default|GetFireball1)) "Undefined" "MultiplyWithRoot" 0 0))
    (:then_1
      (Game|SpawnActorfromClass "/Game/Monster/BP_Fireball.BP_Fireball_C" (Transformation|GetWorldTransform (Variables|Default|GetFireball2)) "Undefined" "MultiplyWithRoot" 0 0))
    (:then_2
      (Game|SpawnActorfromClass "/Game/Monster/BP_Fireball.BP_Fireball_C" (Transformation|GetWorldTransform (Variables|Default|GetFireball3)) "Undefined" "MultiplyWithRoot" 0 0))))