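; BP_Warrior is an AI-controlled melee monster that attacks and damages the VR player.
; On possession by BP_MonsterBP, a looping timer polls the blackboard's monster state.
; The Attack state plays a montage and moves a hit box, with CanAttack blocking re-triggers until MontageEnd clears it and resets the box.
; Box overlap with a VRPlayerPawn applies damage and prints its current health.
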(event OnComponentBeginOverlap(Box)
  (params (OverlappedComponent :type Primitive%20Component%20Object%20Reference) (OtherActor :type Actor%20Object%20Reference) (OtherComp :type Primitive%20Component%20Object%20Reference) (OtherBodyIndex :type Integer) (bFromSweep :type Boolean) (SweepResult :type Hit%20Result%20Structure%20%28by%20ref%29))
  (bind _asvrplayer_pawn (Utilities|Casting|CastToVRPlayerPawn OtherActor))
  (Default|TakeDamage _asvrplayer_pawn (Variables|Default|GetDamage))
  (Development|PrintString (Utilities|String|ToString(Integer) (Variables|/Game/VRTemplate/Blueprints/VRPlayerPawn.VRPlayerPawn_C|GetCurrentHealth _asvrplayer_pawn))))

(event EventBeginPlay
  (|CallParentFunction))

(event Collision|EventActorBeginOverlap
  (params (OtherActor :type Actor%20Object%20Reference))
  (|CallParentFunction OtherActor) ; This node is disabled and will not be called.\nDrag off pins to build functionality.
)

(event EventTick
  (params (DeltaSeconds :type Float%20%28single-precision%29))
  (|CallParentFunction DeltaSeconds) ; This node is disabled and will not be called.\nDrag off pins to build functionality.
)

(event EventPossessed
  (params (NewController :type Controller%20Object%20Reference))
  (Utilities|Casting|CastToBP_MonsterBP NewController)
  (EventDispatchers|BindEventtoOnMontageEnded (Components|SkeletalMesh|GetAnimInstance (Variables|Character|GetMesh)) (EventDispatchers|CreateEvent :!event MontageEnd))
  (Utilities|Time|SetTimerbyFunctionName 0 "UpdateAITick" 0.1 true))

(fn ConstructionScript
  (|CallParentFunction))

(fn UpdateAITick
  (bind _asbp_monster_bp (Utilities|Casting|CastToBP_MonsterBP (Pawn|GetController)))
  (Utilities|IsValid (AI|GetBlackboard _asbp_monster_bp)
    (:Is%20Valid
      (bind _output_get (Variables|Default|SetMonsterState (Utilities|Enum|ByteToEnumEN_Monster (Class|BlackboardComponent|GetValueasEnum (AI|GetBlackboard _asbp_monster_bp) (Utilities|Name|MakeLiteralName "Monster")))))
      (switch Utilities|FlowControl|Switch|SwitchonEN_Monster _output_get
        (:NewEnumerator2
          (if (not (Variables|Default|GetCanAttack))
            (Variables|Default|SetCanAttack true)
            (Animation|PlayAnimMontage (Variables|Default|GetAttackMontage) 1.0 "None")
            (Transformation|SetRelativeLocation (Variables|Default|GetBox) (Math|Vector|MakeVector 0.0 5e+01 89.0) false false)))))))

(fn MontageEnd
  (params (Montage :type Anim%20Montage%20Object%20Reference) (bInterrupted :type Boolean))
  (Variables|Default|SetCanAttack false)
  (Transformation|SetRelativeLocation (Variables|Default|GetBox) (Math|Vector|MakeVector 0.0 0.0 0.0) false false))