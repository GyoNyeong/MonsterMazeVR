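; BP_MonsterBP is an AI controller for monsters that selects a behavior tree by the possessed pawn's class.
; On possession it runs BT_Warrior for BP_Warrior pawns and BT_Mage for BP_Mage pawns.
; AI Perception updates feed the blackboard: a sensed actor becomes TargetActor and switches the Monster state enum.
; A failed sense clears TargetActor and sets the enum to its first state.
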(event OnTargetPerceptionUpdated(AIPerception)
  (params (Actor :type Actor%20Object%20Reference) (Stimulus :type AI%20Stimulus%20Structure))
  (if (.bSuccessfullySensed (Utilities|Struct|BreakAIStimulus Stimulus))
    (AI|Components|Blackboard|SetValueasObject (AI|GetBlackboard 0) (Utilities|Name|MakeLiteralName "TargetActor") Actor)
    (AI|Components|Blackboard|SetValueasEnum (AI|GetBlackboard 0) (Utilities|Name|MakeLiteralName "Monster") (Utilities|Enum|LiteralenumEN_Monster "NewEnumerator2"))
    (else
      (AI|Components|Blackboard|SetValueasObject (AI|GetBlackboard 0) (Utilities|Name|MakeLiteralName "TargetActor") 0)
      (AI|Components|Blackboard|SetValueasEnum (AI|GetBlackboard 0) (Utilities|Name|MakeLiteralName "Monster") (Utilities|Enum|LiteralenumEN_Monster "NewEnumerator0")))))

(event EventBeginPlay)

(event EventPossess
  (params (PossessedPawn :type Pawn%20Object%20Reference))
  (Utilities|FlowControl|Sequence
    (:then_0
      (Utilities|Casting|CastToBP_Warrior PossessedPawn)
      (AI|RunBehaviorTree "/Game/Monster/BT_Warrior.BT_Warrior"))
    (:then_1
      (Utilities|Casting|CastToBP_Mage PossessedPawn)
      (AI|RunBehaviorTree "/Game/Monster/BT_Mage.BT_Mage"))))

(fn ConstructionScript)